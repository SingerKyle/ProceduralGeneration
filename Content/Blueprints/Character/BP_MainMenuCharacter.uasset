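; BP_MainMenuCharacter is a character that can ride ziplines.
; InteractZipline stores line data, and Tick attaches the character once its hands are vertically near the detection point, with wider tolerance unless falling.
; It switches to Flying and eases the capsule toward the end selected by facing direction, faster downhill.
; StopZipline halts that move, while completing it restores Walking.
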(event `StopZipline`
  (bind (_zipline_detection_point_0_x _zipline_detection_point_0_y _zipline_detection_point_0_z) (`KismetMathLibrary.BreakVector` (`self.Zipline Detection Point_0`)))
  (bind _capsulecomponent (`self.CapsuleComponent`))
  (bind (_relativerotation_roll _relativerotation_pitch _relativerotation_yaw) (`KismetMathLibrary.BreakRotator` (`SceneComponent.RelativeRotation` _capsulecomponent)))
  (bind _returnvalue (`KismetMathLibrary.SelectVector` (`self.Zipline End Location_0`) (`self.Zipline Start Location_0`) (>= (`KismetMathLibrary.Dot_VectorVector` (`self.GetActorForwardVector`) (`self.Start Forward_0`)) 0.0)))
  (bind _returnvalue_2 (- _returnvalue (`KismetMathLibrary.MakeVector` 0.0 0.0 (`self.ZiplineHeightOffset_0`))))
  (goto _label :!via `Stop`))

(event `self.ReceiveTick`
  (params (DeltaSeconds :type "Float (single-precision)"))
  (bind (_zipline_detection_point_0_x _zipline_detection_point_0_y _zipline_detection_point_0_z) (`KismetMathLibrary.BreakVector` (`self.Zipline Detection Point_0`)))
  (bind _mesh (`self.Mesh`))
  (bind _capsulecomponent (`self.CapsuleComponent`))
  (bind _zipline_detection_point_0 (`self.Zipline Detection Point_0`))
  (bind (_relativerotation_roll _relativerotation_pitch _relativerotation_yaw) (`KismetMathLibrary.BreakRotator` (`SceneComponent.RelativeRotation` _capsulecomponent)))
  (bind (_velocity_x _velocity_y _velocity_z) (`KismetMathLibrary.BreakVector` (`MovementComponent.Velocity` (`self.CharacterMovement`))))
  (bind _returnvalue (`KismetMathLibrary.SelectVector` (`self.Zipline End Location_0`) (`self.Zipline Start Location_0`) (>= (`KismetMathLibrary.Dot_VectorVector` (`self.GetActorForwardVector`) (`self.Start Forward_0`)) 0.0)))
  (bind (_returnvalue_x _returnvalue_y _returnvalue_z) (`KismetMathLibrary.BreakVector` (- (`self.Zipline Detection Point_0`) (/ (+ (`SceneComponent.GetSocketLocation` _mesh "hand_l") (`SceneComponent.GetSocketLocation` _mesh "hand_r")) 2.0))))
  (bind _returnvalue_2 (- _returnvalue (`KismetMathLibrary.MakeVector` 0.0 0.0 (`self.ZiplineHeightOffset_0`))))
  (`|ExecutionSequence`
    (:`then_0`
      (if (`self.Player Detected_0`)
        (if (< (`KismetMathLibrary.Abs` _returnvalue_z) (`KismetMathLibrary.SelectFloat` 60.0 100.0 (< _velocity_z 0.0)))
          (`CharacterMovementComponent.SetMovementMode` (`self.CharacterMovement`) "MOVE_Flying" 0)
          (`KismetSystemLibrary.MoveComponentTo` (`self.CapsuleComponent`) (- _zipline_detection_point_0 (`KismetMathLibrary.MakeVector` 0.0 0.0 (`self.ZiplineHeightOffset_0`))) (`KismetMathLibrary.FindLookAtRotation` _zipline_detection_point_0 _returnvalue) false false 0.4)
          (set `self.OnZipline_0` true)
          (`KismetSystemLibrary.MoveComponentTo` _capsulecomponent _returnvalue_2 (`KismetMathLibrary.MakeRotator` _relativerotation_roll 0.0 _relativerotation_yaw) false true (/ (`KismetMathLibrary.Vector_Distance` _returnvalue_2 (`self.Zipline Detection Point_0`)) (`KismetMathLibrary.SelectFloat` 1200.0 800.0 (> (- _zipline_detection_point_0_z (.z _returnvalue)) 0.0))) true :!label _label)
          (`CharacterMovementComponent.SetMovementMode` (`self.CharacterMovement`) "MOVE_Walking" 0))))))

(event `self.Interact Zipline`
  (params (bPlayerDetected :type Boolean) (ZiplineDetectionPoint :type "Vector Structure") (ZiplineStartLocation :type "Vector Structure") (ZiplineEndLocation :type "Vector Structure") (StartForward :type "Vector Structure"))
  (set `self.Player Detected_0` bPlayerDetected)
  (set `self.Zipline Detection Point_0` ZiplineDetectionPoint)
  (set `self.Zipline Start Location_0` ZiplineStartLocation)
  (set `self.Zipline End Location_0` ZiplineEndLocation)
  (set `self.Start Forward_0` StartForward))

(fn `UserConstructionScript`)
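; Test zipline actor with a cable between start and end points that reports possible attach positions to overlapping actors.
; Construction places the end mesh and builds a spline mesh, offset below the line, as the overlap volume.
; Overlap starts short timers: one projects the actor's horizontal distance from the start along the cable and sends that point through InteractZiplineMessage.
; End overlap sends a clearing message and cancels timers; CheckDistance is empty.
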(event `self.ReceiveBeginPlay`
  (bind _cable (`self.Cable`))
  (bind _cablecollision (`self.CableCollision`))
  (`SceneComponent.K2_SetWorldLocation` _cable (`SceneComponent.K2_GetComponentLocation` (`self.StartPoint`)) false false)
  (`CableComponent.SetAttachEndToComponent` _cable (`self.EndPoint`) "None")
  (add `PrimitiveComponent.OnComponentBeginOverlap` _cablecollision (delegate `OnPlayerDetected`))
  (add `PrimitiveComponent.OnComponentEndOverlap` _cablecollision (delegate `StopPlayerCheck`)))

(event `OnPlayerDetected`
  (params (OverlappedComponent :type "PrimitiveComponent Object Reference") (OtherActor :type "Actor Object Reference") (OtherComp :type "PrimitiveComponent Object Reference") (OtherBodyIndex :type Integer) (bFromSweep :type Boolean) (SweepResult :type "HitResult Structure (by ref)"))
  (bind _returnvalue (`KismetSystemLibrary.K2_SetTimerDelegate` (delegate `Set Current Target`) 0.05))
  (bind _returnvalue_2 (`KismetSystemLibrary.K2_SetTimerDelegate` (delegate `Check Distance`) 0.05)))

(event `StopPlayerCheck`
  (params (OverlappedComponent :type "PrimitiveComponent Object Reference") (OtherActor :type "Actor Object Reference") (OtherComp :type "PrimitiveComponent Object Reference") (OtherBodyIndex :type Integer))
  (message `/Game/Blueprints/Zipline/BPI_Zipline.Interact Zipline` OtherActor false (0.0 0.0 0.0) (0.0 0.0 0.0) (0.0 0.0 0.0) (0.0 0.0 0.0))
  (`KismetSystemLibrary.K2_ClearAndInvalidateTimerHandle` (stale `OnPlayerDetected` _returnvalue))
  (`KismetSystemLibrary.K2_ClearAndInvalidateTimerHandle` (stale `OnPlayerDetected` _returnvalue_2)))

(event `Set Current Target`
  (bind (_startpoint _endpoint) (`self.GetStartandEndSockets`))
  (bind (_startpoint_2 _endpoint_2) (`self.GetStartandEndSockets`))
  (bind (_returnvalue_x _returnvalue_y) (`KismetMathLibrary.BreakVector` (`SceneComponent.K2_GetComponentLocation` (`self.StartPoint`))))
  (bind (_returnvalue_x_2 _returnvalue_y_2) (`KismetMathLibrary.BreakVector` (`self.K2_GetActorLocation` (stale `OnPlayerDetected` OtherActor))))
  (bind _output_get (set `self.TargetStartPoint` (+ (* (`KismetMathLibrary.GetDirectionUnitVector` _startpoint _endpoint) (`KismetMathLibrary.VSize` (- (`KismetMathLibrary.MakeVector` _returnvalue_x_2 _returnvalue_y_2) (`KismetMathLibrary.MakeVector` _returnvalue_x _returnvalue_y)))) _startpoint)))
  (message `/Game/Blueprints/Zipline/BPI_Zipline.Interact Zipline` (stale `OnPlayerDetected` OtherActor) true _output_get _startpoint_2 _endpoint_2 (`SceneComponent.GetForwardVector` (`self.StartMesh`))))

(event `Check Distance`)

(fn `GetStartandEndSockets`
  (returns (StartPoint :type "Vector Structure") (Endpoint :type "Vector Structure"))
  (return (`SceneComponent.K2_GetComponentLocation` (`self.StartPoint`)) (`SceneComponent.K2_GetComponentLocation` (`self.EndPoint`))))

(fn `UserConstructionScript`
  (bind _spline (`self.Spline`))
  (bind _spline_2 (`self.Spline`))
  (bind _output_get (set `self.EndLocation` (`self.EndLocation`)))
  (`SceneComponent.K2_SetRelativeLocation` (`self.EndMesh`) _output_get false false)
  (`SplineComponent.SetLocationAtSplinePoint` _spline 0 (`SceneComponent.K2_GetComponentLocation` (`self.StartPoint`)) "World" true)
  (`SplineComponent.SetLocationAtSplinePoint` _spline 1 (`SceneComponent.K2_GetComponentLocation` (`self.EndPoint`)) "World" true)
  (for _index (range (+ (- (`SplineComponent.GetNumberOfSplinePoints` (`self.Spline`)) 2) 1))
    (bind _returnvalue (`AddComponent|NODE_AddSplineMeshComponent-0`))
    (set `self.CableCollision` _returnvalue)
    (bind _returnvalue_2 (+ _index 1))
    (`SplineMeshComponent.SetStartAndEnd` _returnvalue (- (`SplineComponent.GetLocationAtSplinePoint` _spline_2 _index "Local") (`KismetMathLibrary.MakeVector` 0.0 0.0 50.0)) (`SplineComponent.GetTangentAtSplinePoint` _spline_2 _index "Local") (- (`SplineComponent.GetLocationAtSplinePoint` _spline_2 _returnvalue_2 "Local") (`KismetMathLibrary.MakeVector` 0.0 0.0 50.0)) (`SplineComponent.GetTangentAtSplinePoint` _spline_2 _returnvalue_2 "Local") true)))